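; BP_DamageZone is a damage zone actor that hurts the first-person player over time while they stay inside its DamageBox.
; Begin overlap stores the player reference and starts a looping one-second timer, intended to drive ApplyDamage, which passes DamagePerSeconds to the player's TakeDamage.
; End overlap clears the timer, so damage relies on overlap events and a timer instead of Tick.
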(event `self.DamageBox.OnComponentBeginOverlap`
  (params (OverlappedComponent :type "PrimitiveComponent Object Reference") (OtherActor :type "Actor Object Reference") (OtherComp :type "PrimitiveComponent Object Reference") (OtherBodyIndex :type Integer) (bFromSweep :type Boolean) (SweepResult :type "HitResult Structure (by ref)"))
  (bind _asbp_first_person_character (cast `/Game/FirstPerson/Blueprints/BP_FirstPersonCharacter` OtherActor))
  (set `self.PlayerRef` _asbp_first_person_character)
  (set `self.bPlayerinside` true)
  (bind _returnvalue (`KismetSystemLibrary.K2_SetTimerDelegate` (`|CreateDelegate` :!event `ApplyDamage`) 1.0 true))
  (set `self.DamageTimer` _returnvalue))

(event `self.DamageBox.OnComponentEndOverlap`
  (params (OverlappedComponent :type "PrimitiveComponent Object Reference") (OtherActor :type "Actor Object Reference") (OtherComp :type "PrimitiveComponent Object Reference") (OtherBodyIndex :type Integer))
  (cast `/Game/FirstPerson/Blueprints/BP_FirstPersonCharacter` OtherActor)
  (set `self.bPlayerinside` false)
  (`KismetSystemLibrary.K2_ClearAndInvalidateTimerHandle` (`self.DamageTimer`)))

(event `ApplyDamage`
  (`/Game/FirstPerson/Blueprints/BP_FirstPersonCharacter.TakeDamage` (`self.PlayerRef`) (`self.DamagePerSeconds`)))

(fn `UserConstructionScript`)